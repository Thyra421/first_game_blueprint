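; BP_GameManager is a game manager actor that keeps an elapsed-time counter and creates the score UI.
; On BeginPlay it starts a looping one-second timer on TickTimer, which adds a second to the Timer variable.
; It also adds a WB_Score widget to the viewport, passing itself as the widget's GameManager reference.
; ResetTimer sets Timer back to a zeroed DateTime.
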(event EventBeginPlay
  (Utilities|FlowControl|Sequence
    (:then_0
      (Utilities|Time|SetTimerbyFunctionName 0 "TickTimer" 1.0 true))
    (:then_1
      (bind _returnvalue (UserInterface|CreateWidget "/Game/WB_Score.WB_Score_C"))
      (Variables|/Game/WB_Score.WB_Score_C|SetGameManager _returnvalue self)
      (UserInterface|Viewport|AddtoViewport _returnvalue 0))))

(event Collision|EventActorBeginOverlap
  (params (OtherActor :type Actor%20Object%20Reference)))

(event EventTick
  (params (DeltaSeconds :type Float%20%28single-precision%29)))

(fn ConstructionScript)

(fn ResetTimer
  (Variables|Default|SetTimer (Math|DateTime|MakeDateTime 0 0 0)))

(fn TickTimer
  (Variables|Default|SetTimer (+ (Variables|Default|GetTimer) (Math|Timespan|FromSeconds 1.0))))