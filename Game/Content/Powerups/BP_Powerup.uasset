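; BP_Powerup is a base pickup that reacts when a BP_Paladin actor overlaps it.
; On overlap it spawns a BP_NS_Energy_2_Blueprint effect at Sphere1's transform, calls Trigger, adds a fixed score through the paladin's GameManager, then destroys itself.
; Trigger is the hook for child powerups to override with their own effect; the base version only prints a warning that it must be overridden.
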(event Custom|Trigger
  (Development|PrintString "Trigger must be overriden"))

(event Collision|EventActorBeginOverlap
  (params (OtherActor :type Actor%20Object%20Reference))
  (bind _asbp_paladin (Utilities|Casting|CastToBP_Paladin OtherActor))
  (Utilities|IsValid _asbp_paladin
    (:Is%20Valid
      (Utilities|FlowControl|Sequence
        (:then_0
          (Game|SpawnActorfromClass "/Game/sA_PickupSet_1/Fx/NiagaraSystems/BP_NS_Energy_2_Blueprint.BP_NS_Energy_2_Blueprint_C" (Transformation|GetWorldTransform (Variables|Default|GetSphere1)) "Undefined" "MultiplyWithRoot" 0 0))
        (:then_1
          (CallFunction|Trigger))
        (:then_2
          (Default|AddScore (Variables|/Game/Characters/Paladin/BP_Paladin.BP_Paladin_C|GetGameManager _asbp_paladin) 25))
        (:then_3
          (Actor|DestroyActor))))))

(fn ConstructionScript)