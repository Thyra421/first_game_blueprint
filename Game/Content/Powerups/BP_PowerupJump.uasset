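; BP_PowerupJump is a powerup that gives the player's Paladin character its jump powerup.
; Its Trigger event casts player character 0 to BP_Paladin, calls PowerupJump on it and plays a 2D powerup sound.
; The effect itself lives in BP_Paladin, and nothing in this graph calls Trigger or handles overlap.
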(event EventBeginPlay
  (|CallParentFunction) ; This node is disabled and will not be called.\nDrag off pins to build functionality.
)

(event Collision|EventActorBeginOverlap
  (params (OtherActor :type Actor%20Object%20Reference))
  (|CallParentFunction OtherActor) ; This node is disabled and will not be called.\nDrag off pins to build functionality.
)

(event EventTick
  (params (DeltaSeconds :type Float%20%28single-precision%29))
  (|CallParentFunction DeltaSeconds) ; This node is disabled and will not be called.\nDrag off pins to build functionality.
)

(event EventTrigger
  (bind _asbp_paladin (Utilities|Casting|CastToBP_Paladin (Game|GetPlayerCharacter 0)))
  (Default|PowerupJump _asbp_paladin)
  (Audio|PlaySound2D "/Game/Powerups/powerup.powerup" 1.0 1.0 0.0 0 0))

(fn ConstructionScript
  (|CallParentFunction))