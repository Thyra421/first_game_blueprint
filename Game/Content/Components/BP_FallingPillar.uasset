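; BP_FallingPillar is a pillar actor that topples when a BP_Fireball overlaps it.
; BeginPlay stores the starting rotation, and the overlap latches a ShouldFall flag.
; While the flag is set, Tick lerps the current rotation toward a fixed tilted pitch, using the starting roll and yaw.
; The alpha is delta time times FallingSpeed, so the fall eases out rather than simulating physics.
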(event EventBeginPlay
  (Variables|Default|SetInitialRotation (Transformation|GetActorRotation)))

(event Collision|EventActorBeginOverlap
  (params (OtherActor :type Actor%20Object%20Reference))
  (Utilities|Casting|CastToBP_Fireball OtherActor)
  (Variables|Default|SetShouldFall true))

(event EventTick
  (params (DeltaSeconds :type Float%20%28single-precision%29))
  (bind _initialrotation (Variables|Default|GetInitialRotation))
  (bind (_roll _pitch _yaw) (Math|Rotator|BreakRotator _initialrotation))
  (if (Variables|Default|GetShouldFall)
    (Transformation|SetActorRotation (Math|Rotator|Lerp(Rotator) (Transformation|GetActorRotation) (Math|Rotator|CombineRotators "0, 0, 0" (Math|Rotator|MakeRotator _roll -72.0 _yaw)) (* DeltaSeconds (Variables|Default|GetFallingSpeed))))))

(fn ConstructionScript)