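; BP_NPC is an AI character that knocks the player's Paladin into the air when it comes close.
; BeginPlay caches the player, then Tick checks proximity and, if pushing is allowed, sphere-traces for pawns along the NPC's FollowCamera forward vector.
; A Paladin hit is launched forward and up with a sound and backhand montage, while a timer calls ResetCooldown to re-enable pushing.
; Destruction plays a pain sound.
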(event OnComponentHit(CapsuleComponent)
  (params (HitComponent :type Primitive%20Component%20Object%20Reference) (OtherActor :type Actor%20Object%20Reference) (OtherComp :type Primitive%20Component%20Object%20Reference) (NormalImpulse :type Vector :default "0, 0, 0") (Hit :type Hit%20Result%20Structure%20%28by%20ref%29)))

(event EventBeginPlay
  (bind _asbp_paladin (Utilities|Casting|CastToBP_Paladin (Game|GetPlayerCharacter 0)))
  (Variables|Default|SetPlayer _asbp_paladin))

(event Collision|EventActorBeginOverlap
  (params (OtherActor :type Actor%20Object%20Reference)))

(event EventTick
  (params (DeltaSeconds :type Float%20%28single-precision%29))
  (bind _followcamera (Variables|Default|GetFollowCamera))
  (bind _followcamera_2 (Variables|Default|GetFollowCamera))
  (bind _returnvalue (Transformation|GetWorldRotation _followcamera))
  (bind _returnvalue_2 (Transformation|GetWorldLocation _followcamera_2))
  (bind _returnvalue_3 (Math|Vector|GetForwardVector _returnvalue))
  (bind _returnvalue_4 (* _returnvalue_3 1e+03))
  (if (< (Math|Vector|Distance(Vector) (Transformation|GetActorLocation (Variables|Default|GetPlayer)) (Transformation|GetActorLocation self)) 1e+02)
    (if (Variables|Default|GetCanPush)
      (bind (_outhit _returnvalue_5) (Collision|SphereTraceForObjects _returnvalue_2 (+ _returnvalue_2 (* (Math|Vector|GetForwardVector (Transformation|GetWorldRotation _followcamera_2)) 1e+03)) 3e+01 (Utilities|Array|MakeArray "ObjectTypeQuery3") false 0 "None"))
      (if _returnvalue_5
        (bind _asbp_paladin (Utilities|Casting|CastToBP_Paladin (.HitActor (Collision|BreakHitResult _outhit))))
        (Character|LaunchCharacter _asbp_paladin (Math|Vector|MakeVector (.x _returnvalue_4) (.y _returnvalue_4) (+ (.z _returnvalue_4) 7e+02)) false false)
        (Utilities|FlowControl|Sequence
          (:then_0
            (Audio|PlaySound2D "/Game/Characters/AI/SoundEffects/boing.boing" 1.0 1.0 0.0 0 0))
          (:then_1
            (Variables|Default|SetCanPush false)
            (Utilities|Time|SetTimerbyFunctionName 0 "ResetCooldown" (Variables|Default|GetCooldown)))
          (:then_2
            (Animation|PlayAnimMontage "/Game/Characters/AI/Standing_Melee_Attack_Backhand__1__Montage.Standing_Melee_Attack_Backhand__1__Montage" 1.0 "None")))))))

(event EventDestroyed
  (Audio|PlaySound2D "/Game/Characters/AI/SoundEffects/pain.pain" 1.0 1.0 0.0 0 0))

(fn ConstructionScript)

(fn ResetCooldown
  (Variables|Default|SetCanPush true))